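; BP_Zombie is an AI-controlled zombie enemy that damages the player character on touch.
; On spawn it randomizes mesh scale, yaw and walk speed for variety.
; Overlapping its capsule collision lowers the player's Health after a short delay.
; Kill stops the AI's brain logic, ragdolls the mesh, disables capsule collision, then broadcasts OnKilled and destroys the actor after a delay.
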(event `self.CapsuleCollison.OnComponentBeginOverlap`
  (params (OverlappedComponent :type "PrimitiveComponent Object Reference") (OtherActor :type "Actor Object Reference") (OtherComp :type "PrimitiveComponent Object Reference") (OtherBodyIndex :type Integer) (bFromSweep :type Boolean) (SweepResult :type "HitResult Structure (by ref)"))
  (bind _asue_4asp_character (cast `/Game/Player/Ue4ASP_Character` OtherActor))
  (`KismetSystemLibrary.Delay` 0.5)
  (set `/Game/Player/Ue4ASP_Character.Health` (- (`/Game/Player/Ue4ASP_Character.Health` _asue_4asp_character) 0.2) _asue_4asp_character))

(event `self.ReceiveBeginPlay`
  (bind _returnvalue (`KismetMathLibrary.RandomFloatInRange` 0.9 1.1))
  (`SceneComponent.SetWorldScale3D` (`self.Mesh`) (`KismetMathLibrary.MakeVector` _returnvalue _returnvalue _returnvalue))
  (`self.K2_SetActorRotation` (`KismetMathLibrary.MakeRotator` 0.0 0.0 (`KismetMathLibrary.RandomFloatInRange` 0.0 360.0)))
  (set `CharacterMovementComponent.MaxWalkSpeed` (`KismetMathLibrary.RandomFloatInRange` 200.0 600.0) (`self.CharacterMovement`)))

(event `Kill`
  (bind _mesh (`self.Mesh`))
  (`BrainComponent.StopLogic` (`AIController.BrainComponent` (`AIBlueprintHelperLibrary.GetAIController` self)) "")
  (`PrimitiveComponent.SetCollisionProfileName` _mesh "Ragdoll" true)
  (`PrimitiveComponent.SetSimulatePhysics` _mesh true)
  (`PrimitiveComponent.SetCollisionProfileName` (`self.CapsuleComponent`) "NoCollision" true)
  (`KismetSystemLibrary.Delay` 5.0)
  (`self.OnKilled` self)
  (`self.K2_DestroyActor`))

(fn `UserConstructionScript`)