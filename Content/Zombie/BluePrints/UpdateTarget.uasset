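; Behavior Tree service that decides whether a zombie chases the player based on proximity.
; Each AI tick it compares the squared distance between the pawn and player character 0 against the squared perception distance, with no sight check.
; In range, it writes the player to the target Blackboard key and sets the chase state; otherwise it clears the target and resets the state.
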(event `self.ReceiveTickAI`
  (params (OwnerController :type "AIController Object Reference") (ControlledPawn :type "Pawn Object Reference") (DeltaSeconds :type "Float (single-precision)"))
  (if (< (`KismetMathLibrary.Vector_DistanceSquared` (`Actor.K2_GetActorLocation` ControlledPawn) (`Actor.K2_GetActorLocation` (`GameplayStatics.GetPlayerCharacter` 0))) (`KismetMathLibrary.Square` (`self.PerseptionDistance`)))
    ;[1 1 1] schasing
    (`BTFunctionLibrary.SetBlackboardValueAsObject` (`self.AI_Target`) (`GameplayStatics.GetPlayerCharacter` 0))
    (`BTFunctionLibrary.SetBlackboardValueAsEnum` (`self.AI_State`) (enumliteral `/Game/Zombie/BluePrints/ZombieAIState` "NewEnumerator1"))
    (else
      ;[1 1 1] stop chasing
      (`BTFunctionLibrary.SetBlackboardValueAsObject` (`self.AI_Target`))
      (`BTFunctionLibrary.SetBlackboardValueAsEnum` (`self.AI_State`) (enumliteral `/Game/Zombie/BluePrints/ZombieAIState` "NewEnumerator0")))))